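; Clickable cube spawner that creates friendly or enemy test troops, with a point light for mouse feedback.
; Hovering on or off toggles the light's visibility; clicking turns it red and releasing turns it blue.
; A click spawns the troop class chosen by Friendly, offset to either side along X, passing in health, speed, fire rate and spot radius.
; A DelayCounter flag around a Delay blocks further spawns during SpawnCooldown.
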(event `self.ReceiveBeginPlay`
  (set `self.DelayCounter` false))

(event `self.Cube.OnBeginCursorOver`
  (params (TouchedComponent :type "PrimitiveComponent Object Reference"))
  (`SceneComponent.ToggleVisibility` (`self.PointLight`) false :!label _label))

(event `self.Cube.OnEndCursorOver`
  (params (TouchedComponent :type "PrimitiveComponent Object Reference"))
  (goto _label))

(event `self.Cube.OnClicked`
  (params (TouchedComponent :type "PrimitiveComponent Object Reference") (ButtonPressed :type "Key Structure"))
  (`LightComponent.SetLightColor` (`self.PointLight`) (struct :`R` 1.0 :`G` 0.014303 :`A` 1.0) true)
  (if (`self.DelayCounter`)
    _
    (elif (`self.Friendly`)
      (`|SpawnActorFromClass` "/Game/Scripts/Testing_troop.Testing_troop_C" (`KismetMathLibrary.MakeTransform` (+ (`SceneComponent.K2_GetComponentLocation` (`self.Cube`)) (150.0 0.0 30.0))) "AlwaysSpawn" "OverrideRootScale" null (`self.Spot_Radius`) (`self.Health`) (`self.Troop_Speed`) (`self.Fire Rate`) null)
      (set `self.DelayCounter` true)
      (`KismetSystemLibrary.Delay` (`self.Spawn_Cooldown`))
      (set `self.DelayCounter` false)
      (else
        (`|SpawnActorFromClass` "/Game/Scripts/Testing_troop_enemy.Testing_troop_enemy_C" (`KismetMathLibrary.MakeTransform` (+ (`SceneComponent.K2_GetComponentLocation` (`self.Cube`)) (-150.0 0.0 30.0))) "AlwaysSpawn" "OverrideRootScale" null (`self.Spot_Radius`) (`self.Troop_Speed`) (`self.Fire Rate`) (`self.Health`) null)
        (set `self.DelayCounter` true)
        (`KismetSystemLibrary.Delay` (`self.Spawn_Cooldown`))
        (set `self.DelayCounter` false)))))

(event `self.Cube.OnReleased`
  (params (TouchedComponent :type "PrimitiveComponent Object Reference") (ButtonReleased :type "Key Structure"))
  (`LightComponent.SetLightColor` (`self.PointLight`) (struct :`G` 0.369965 :`B` 1.0 :`A` 1.0) true))

(fn `UserConstructionScript`)